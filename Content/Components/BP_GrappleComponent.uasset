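; Grapple component that shows an on-screen icon over the best valid grapple point available to its owner.
; Creates the icon widget at BeginPlay, then each Tick queries GetBestValidGrapplePoint and adds or removes the widget as validity changes.
; The icon follows the point's projected screen position plus an offset.
; Owner-to-point distance, normalized over GrappleRange, drives a curve that sets icon scale within IconScaleRange.
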(event `self.ReceiveBeginPlay`
  ;[1 1 1] Create GrappleIcon Widget
  (bind _returnvalue (`|CreateWidget` "/Game/UI/WBP_GrappleIcon.WBP_GrappleIcon_C" (`GameplayStatics.GetPlayerController` 0)))
  (set `self.IconWidget` _returnvalue))

(event `self.ReceiveTick`
  (params (DeltaSeconds :type "Float (single-precision)"))
  (`self.UpdateGrappleIcon`))

(fn `UpdateGrappleIcon`
  (locals (BestValidGP :type "GrapplePoint Object Reference"))
  (bind _iconscalerange (`self.IconScaleRange`))
  (bind _grapplerange (`self.GrappleRange`))
  (bind (_screenposition _returnvalue) (`GameplayStatics.ProjectWorldToScreen` (`GameplayStatics.GetPlayerController` 0) (`Actor.K2_GetActorLocation` (`local.BestValidGP`)) true))
  (bind _returnvalue_2 (`self.GetBestValidGrapplePoint`))
  (bind _output_get (set `local.BestValidGP` _returnvalue_2))
  (`/Engine/EditorBlueprintResources/StandardMacros.IsValid` _output_get
    (:`Is Valid`
      ;[1 1 1] If not, add to viewport
      (if (not (`Widget.IsInViewport` (`self.IconWidget`)))
        (`UserWidget.AddToViewport` (`self.IconWidget`) 0))
      ;[1 1 1] Set Icon screen pos based on GP world pos
      (`UserWidget.SetPositionInViewport` (`self.IconWidget`) (+ _screenposition (`KismetMathLibrary.Conv_VectorToVector2D` (`self.IconOffset`))) _returnvalue)
      ;[1 1 1] Set Icon scale based on Hero distance to GP
      (`Widget.SetRenderScale` (`self.IconWidget`) (* (1.0 1.0) (`KismetMathLibrary.MapRangeClamped` (`CurveFloat.GetFloatValue` (`self.IconDistanceScaleCurve`) (`KismetMathLibrary.MapRangeClamped` (`KismetMathLibrary.Vector_Distance` (`Actor.K2_GetActorLocation` (`local.BestValidGP`)) (`Actor.K2_GetActorLocation` (`self.GetOwner`))) (`.Value` (break `FloatRangeBound` (break `FloatRange` _grapplerange))) (`.Value` (break `FloatRangeBound` (`.UpperBound` (break `FloatRange` _grapplerange)))) 0.0 1.0)) 0.0 1.0 (`.Value` (break `FloatRangeBound` (break `FloatRange` _iconscalerange))) (`.Value` (break `FloatRangeBound` (`.UpperBound` (break `FloatRange` _iconscalerange))))))))
    (:`Is Not Valid`
      ;[1 1 1] Remove icon from viewport
      (if (`Widget.IsInViewport` (`self.IconWidget`))
        (`Widget.RemoveFromParent` (`self.IconWidget`))))))