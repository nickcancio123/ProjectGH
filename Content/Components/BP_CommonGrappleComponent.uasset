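; Grapple component that displays a screen-space icon over the owner's grapple point.
; Each tick it projects the point's location to the viewport with an offset, hiding the icon when none is valid.
; The icon's render angle doubles as state: zero tracks the best valid point, while spinning tracks the current one.
; Icon scale follows a curve over the eye-to-point distance, normalized to grapple range.
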(event `self.ReceiveBeginPlay`
  (bind _returnvalue (`|CreateWidget` "/Game/UI/WBP_GrappleIcon.WBP_GrappleIcon_C" (`GameplayStatics.GetPlayerController` 0)))
  (set `self.GrappleIcon` _returnvalue))

(event `self.ReceiveTick`
  (params (DeltaSeconds :type "Float (single-precision)"))
  (`self.SetGrappleIconVPPosition`)
  (`self.SetGrappleIconScale`))

(event `self.SpinGrappleIcon`
  (params (DeltaTime :type "Float (single-precision)"))
  (bind _output_get (set `self.GrappleIconAngle` (+ (`self.GrappleIconAngle`) (* DeltaTime (`self.GrappleIconSpinRate`)))))
  (`Widget.SetRenderTransformAngle` (`self.GrappleIcon`) _output_get))

(event `self.ResetGrappleIconAngle`
  (`Widget.SetRenderTransformAngle` (`self.GrappleIcon`) 0.0))

(fn `SetGrappleIconScale`
  (bind (_grapplerange_x _grapplerange_y) (`KismetMathLibrary.BreakVector2D` (`self.GrappleRange`)))
  (bind _grappleiconscalerange (`self.GrappleIconScaleRange`))
  (if (and (`KismetSystemLibrary.IsValid` (`self.GrapplePoint`)) (`Widget.IsInViewport` (`self.GrappleIcon`)))
    (`Widget.SetRenderScale` (`self.GrappleIcon`) (* (1.0 1.0) (`KismetMathLibrary.MapRangeClamped` (`CurveFloat.GetFloatValue` (`self.GrappleIconDistanceScaleCurve`) (`KismetMathLibrary.MapRangeClamped` (`KismetMathLibrary.Vector_Distance` (`Actor.GetActorEyesViewPoint` (`self.GetOwner`)) (`Actor.K2_GetActorLocation` (`self.GrapplePoint`))) _grapplerange_x _grapplerange_y 0.0 1.0)) 0.0 1.0 (`.Value` (break `FloatRangeBound` (break `FloatRange` _grappleiconscalerange))) (`.Value` (break `FloatRangeBound` (`.UpperBound` (break `FloatRange` _grappleiconscalerange)))))))))

(fn `SetGrappleIconVPPosition`
  ;[1 1 1] Check if spinning
  (if (== (`Widget.GetRenderTransformAngle` (`self.GrappleIcon`)) 0.0)
    ;[1 1 1] Check if GP is valid
    (bind _returnvalue (`self.GetBestValidGrapplePoint`))
    (bind _output_get (set `self.GrapplePoint` _returnvalue))
    (if (`KismetSystemLibrary.IsValid` _output_get)
      (if (not (`Widget.IsInViewport` (`self.GrappleIcon`))) :!label _label
        (`UserWidget.AddToViewport` (`self.GrappleIcon`) 0))
      ;[1 1 1] Set position
      (`UserWidget.SetPositionInViewport` (`self.GrappleIcon`) (+ (`WidgetLayoutLibrary.ProjectWorldLocationToWidgetPosition` (`GameplayStatics.GetPlayerController` 0) (`Actor.K2_GetActorLocation` (`self.GrapplePoint`)) true) (`self.GrappleIconVPOffset`)) false)
      (else
        (if (`Widget.IsInViewport` (`self.GrappleIcon`)) :!label _label_2
          (`Widget.RemoveFromParent` (`self.GrappleIcon`)))))
    (else
      (bind _returnvalue_2 (`self.GetCurrentGrapplePoint`))
      (bind _output_get_2 (set `self.GrapplePoint` _returnvalue_2))
      (if (`KismetSystemLibrary.IsValid` _output_get_2)
        (goto _label)
        (else
          (goto _label_2))))))