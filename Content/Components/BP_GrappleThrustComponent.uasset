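; BP_GrappleThrustComponent is an actor component that, by its name, is meant for grapple thrust, though it holds no thrust logic.
; On BeginPlay it looks for a BP_CommonGrappleComponent on its owner, adds one if none exists, and caches the reference.
; It prints a debug string when it finds an existing component, and its Tick is empty.
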(event `self.ReceiveBeginPlay`
  (`self.GetCommonGrappleCompRef`))

(event `self.ReceiveTick`
  (params (DeltaSeconds :type "Float (single-precision)")))

(fn `GetCommonGrappleCompRef`
  (bind _returnvalue (`Actor.GetComponentByClass` (`self.GetOwner`) "/Game/Components/BP_CommonGrappleComponent.BP_CommonGrappleComponent_C"))
  (if (`KismetSystemLibrary.IsValid` _returnvalue)
    (`self.SetCommonGrappleComp` _returnvalue)
    (`KismetSystemLibrary.PrintString` "Created Common Grapple ref")
    (else
      (bind _returnvalue_2 (`|AddComponentByClass` (`self.GetOwner`) "/Game/Components/BP_CommonGrappleComponent.BP_CommonGrappleComponent_C"))
      (`self.SetCommonGrappleComp` _returnvalue_2))))