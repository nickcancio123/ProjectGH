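; A grapple point actor that oscillates back and forth around the location where it begins play.
; BeginPlay stores that start position and adds a phase offset to the angle, so separate instances can move out of sync.
; Each Tick adds delta time to the angle and sets the location along a move direction using its sine scaled by an amplitude, without sweeping.
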(event `self.ReceiveBeginPlay`
  (set `self.StartPos` (`self.K2_GetActorLocation`))
  (set `self.Theta` (+ (`self.Theta`) (`self.ThetaOffset`))))

(event `self.ReceiveTick`
  (params (DeltaSeconds :type "Float (single-precision)"))
  ;[1 1 1] Sinusoidal movement
  (bind _output_get (set `self.Theta` (+ DeltaSeconds (`self.Theta`))))
  (`self.K2_SetActorLocation` (+ (`self.StartPos`) (* (`self.MoveDir`) (* (`KismetMathLibrary.Sin` _output_get) (`self.MoveAmp`))))))

(fn `UserConstructionScript`)